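; Game mode for an FPS level that tracks three missions (fetch, mech destroy, bunker invasion) and relays their state to the mission HUD.
; Update functions store each mission's status and reveal it on MissionWidgetHUD, while others set titles and copy objective active flags.
; BeginPlay caches the pilot character for TimerFunc, a delayed countdown that flags the pilot when finished but is never run from the event graph.
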(event `self.ReceiveBeginPlay`
  (bind _asbp_pilot_character (cast `/Game/FPS/Core/BP_PilotCharacter` (`GameplayStatics.GetPlayerPawn` 0)))
  (set `self.As BP Pilot Character` _asbp_pilot_character))

(event `self.ReceiveTick`
  (params (DeltaSeconds :type "Float (single-precision)")))

(fn `GetMissionsTitles`
  (params (MissionTitle1 :type String) (MissionTitle2 :type String) (MissionTitle3 :type String))
  (`|ExecutionSequence`
    (:`then_0`
      (set `self.MissionTitle1` MissionTitle1)
      (`TextBlock.SetText` (`/Game/Missions/WBP_MissionHUD.ActiveMission1TitleNameText` (`self.MissionWidgetHUD`)) (`KismetTextLibrary.Conv_StringToText` (`self.MissionTitle1`))))
    (:`then_1`
      (set `self.MissionTitle2` MissionTitle2)
      (`TextBlock.SetText` (`/Game/Missions/WBP_MissionHUD.ActiveMission2TitleNameText` (`self.MissionWidgetHUD`)) (`KismetTextLibrary.Conv_StringToText` (`self.MissionTitle2`))))
    (:`then_2`
      (set `self.MissionTitle3` MissionTitle3)
      (`TextBlock.SetText` (`/Game/Missions/WBP_MissionHUD.ActiveMission3TitleNameText` (`self.MissionWidgetHUD`)) (`KismetTextLibrary.Conv_StringToText` (`self.MissionTitle3`))))))

(fn `UpdateMission1(FetchQuest)`
  (params (`Mission 1 Status Text` :type String))
  (set `self.currentMission1StatusText` `Mission 1 Status Text`)
  (`TextBlock.SetText` (`/Game/Missions/WBP_MissionHUD.ActiveMission1StatusText` (`self.MissionWidgetHUD`)) (`KismetTextLibrary.Conv_StringToText` (`self.currentMission1StatusText`)))
  (`Widget.SetVisibility` (`/Game/Missions/WBP_MissionHUD.ActiveMission1StatusScaleBox` (`self.MissionWidgetHUD`)) "Visible"))

(fn `UpdateMission2(MechDestroyQuest)`
  (params (`Mission 2 Status Text` :type String))
  (set `self.currentMission2StatusText` `Mission 2 Status Text`)
  (`TextBlock.SetText` (`/Game/Missions/WBP_MissionHUD.ActiveMission2StatusText` (`self.MissionWidgetHUD`)) (`KismetTextLibrary.Conv_StringToText` (`self.currentMission2StatusText`)))
  (`Widget.SetVisibility` (`/Game/Missions/WBP_MissionHUD.ActiveMission2StatusScaleBox` (`self.MissionWidgetHUD`)) "Visible"))

(fn `UpdateMission3(InvadeBUnker)`
  (params (`Mission 3 Status Text` :type String))
  (set `self.currentMission3StatusText` `Mission 3 Status Text`)
  (`TextBlock.SetText` (`/Game/Missions/WBP_MissionHUD.ActiveMission3StatusText` (`self.MissionWidgetHUD`)) (`KismetTextLibrary.Conv_StringToText` (`self.currentMission3StatusText`)))
  (`Widget.SetVisibility` (`/Game/Missions/WBP_MissionHUD.ActiveMission3StatusScaleBox` (`self.MissionWidgetHUD`)) "Visible"))

(fn `UpdateMissionCompleteHUD`
  (`|ExecutionSequence`
    (:`then_0`
      (if (`self.Obj1Active`)
        (set `/Game/Missions/WBP_MissionHUD.IsObj1Active` true (`self.MissionWidgetHUD`))
        (else
          (set `/Game/Missions/WBP_MissionHUD.IsObj1Active` false (`self.MissionWidgetHUD`)))))
    (:`then_1`
      (if (`self.Obj2Active`)
        (set `/Game/Missions/WBP_MissionHUD.IsObj2Active` true (`self.MissionWidgetHUD`))
        (else
          (set `/Game/Missions/WBP_MissionHUD.IsObj2Active` false (`self.MissionWidgetHUD`)))))
    (:`then_2`
      (if (`self.Obj3Active`)
        (set `/Game/Missions/WBP_MissionHUD.IsObj3Active` true (`self.MissionWidgetHUD`))
        (else
          (set `/Game/Missions/WBP_MissionHUD.IsObj3Active` false (`self.MissionWidgetHUD`)))))))

(fn `UserConstructionScript`)