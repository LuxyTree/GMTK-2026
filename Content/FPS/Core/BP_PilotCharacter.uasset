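; First-person pilot character with parkour movement and a ball that can be picked up, dropped or thrown at three charge levels.
; Enhanced Input forwards jump, sprint and crouch/slide to the ParkourMovement component, whose mode drives timelines for sprint FOV and capsule crouch height.
; Line traces force crouching under obstacles and flag nearby walls.
; Reload toggles a recall flag and resets the level; weapon inventory and holster input are stubs.
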(event `self.ReceiveBeginPlay`
  (bind _returnvalue (`GameplayStatics.GetPlayerCameraManager` 0))
  ;[1 1 1] Initialize Pilot
  (`self.SetupPilotControls`)
  (`self.SpawnInventory`)
  (`self.CreatePilotHUD`)
  (`self.HolsterToggle`)
  (`/Game/FPS/Core/PilotParkourMovement.InitializePilot` (`self.ParkourMovement`) self)
  ;;[1 1 1] Pilot Look Up/Down Max
  (set `PlayerCameraManager.ViewPitchMin` -80.0 _returnvalue)
  (set `PlayerCameraManager.ViewPitchMax` 80.0 _returnvalue))

(event `CreatePilotHUD`
  ;[1 1 1] Create HUD
  (bind _returnvalue (`|CreateWidget` "/Game/FPS/Core/WBP_PilotUI.WBP_PilotUI_C" (`GameplayStatics.GetPlayerController` 0)))
  (`UserWidget.AddToViewport` _returnvalue 0))

(event `self.ReceiveTick`
  (params (DeltaSeconds :type "Float (single-precision)"))
  ;[1 1 1] Update Event
  (`|ExecutionSequence`
    (:`then_0`
      (`self.PilotRotationPivot`)
      (`self.CheckWallDistance`)
      (`self.CameraFOVRun`)
      (set `self.PilotSpeedometer` (`KismetMathLibrary.VSize` (`self.GetVelocity`))))
    (:`then_1`
      (`self.TimerDone`))))

(event `EnhancedInput|/Game/FPS/Data/IA_PilotTest`
  (params (ActionValue :type Boolean) (ElapsedSeconds :type "Float (double-precision)") (TriggeredSeconds :type "Float (double-precision)") (InputAction :type "InputAction Object Reference" :default "/Game/FPS/Data/IA_PilotTest.IA_PilotTest"))
  ;[1 1 1] Update Event
  ;;[1 1 1] Debug (T)
  (:`Triggered`
    (`KismetSystemLibrary.PrintString` "Pilot Test")))

(event `SetupPilotControls`
  ;[1 1 1] Player: Pilot Movement Mechanics
  ;;[1 1 1] Link Correct Movement Mapping (Happens in Player Controller Now)
  (`EnhancedInputSubsystemInterface.AddMappingContext` (pcsubsystem `EnhancedInputLocalPlayerSubsystem` (`GameplayStatics.GetPlayerController` 0)) "/Game/FPS/Data/IMC_Pilot.IMC_Pilot" 0 (struct)))

(event `EnhancedInput|/Game/FPS/Data/IA_PilotCamera`
  (params (ActionValue :type "Vector2D Structure") (ElapsedSeconds :type "Float (double-precision)") (TriggeredSeconds :type "Float (double-precision)") (InputAction :type "InputAction Object Reference" :default "/Game/FPS/Data/IA_PilotCamera.IA_PilotCamera"))
  (bind (_x _y) (`KismetMathLibrary.BreakVector2D` (`self.MouseInput`)))
  ;[1 1 1] Player: Pilot Movement Mechanics
  ;;[1 1 1] Mouse Camera Movement
  (:`Triggered`
    (set `self.MouseInput` ActionValue :!label _label)
    (`self.AddControllerPitchInput` (* _y -1.0))
    (`self.AddControllerYawInput` _x))
  (:`Completed`
    (goto _label)))

(event `PilotRotationPivot`
  ;[1 1 1] Player: Pilot Movement Mechanics
  ;;[1 1 1] Pilot Rotation Pivot (Allows the players arms to move same as the mouse)
  (`SceneComponent.K2_SetRelativeRotation` (`self.Pivot`) (`KismetMathLibrary.MakeRotator` 0.0 (.pitch (`self.GetControlRotation`))) false false))

(event `EnhancedInput|/Game/FPS/Data/IA_PilotMovement`
  (params (ActionValue :type "Vector2D Structure") (ElapsedSeconds :type "Float (double-precision)") (TriggeredSeconds :type "Float (double-precision)") (InputAction :type "InputAction Object Reference" :default "/Game/FPS/Data/IA_PilotMovement.IA_PilotMovement"))
  (bind (_x _y) (`KismetMathLibrary.BreakVector2D` (`self.MoveInput`)))
  ;[1 1 1] Player: Pilot Movement Mechanics
  ;;[1 1 1] WASD Pilot Movement
  (:`Triggered`
    (`|ExecutionSequence`
      (:`then_0`
        (set `self.MoveInput` ActionValue :!label _label_2)
        (`self.AddMovementInput` (* (`self.GetActorForwardVector`) _y))
        (`self.AddMovementInput` (* (`self.GetActorRightVector`) _x))
        (`/Game/FPS/Core/PilotParkourMovement.PilotSpeedConservation` (`self.ParkourMovement`))
        (`KismetSystemLibrary.Delay` (`self.Accel/Decel Determination Time`))
        (set `/Game/FPS/Core/PilotParkourMovement.LastSpeed` (`self.PilotSpeedometer`) (`self.ParkourMovement`)))
      (:`then_1`
        (`/Engine/EditorBlueprintResources/StandardMacros.DoOnce` false
          (:`Completed`
            (`self.TIMERSTART`))))))
  (:`Completed`
    (goto _label_2)))

(event `EnhancedInput|/Game/FPS/Data/IA_PilotJump`
  (params (ActionValue :type Boolean) (ElapsedSeconds :type "Float (double-precision)") (TriggeredSeconds :type "Float (double-precision)") (InputAction :type "InputAction Object Reference" :default "/Game/FPS/Data/IA_PilotJump.IA_PilotJump"))
  ;[1 1 1] Player: Pilot Movement Mechanics
  ;;[1 1 1] Pilot Jumping
  (:`Started`
    (if (not (`/Game/FPS/Core/PilotParkourMovement.bSlideInputDelay` (`self.ParkourMovement`)))
      (`self.Jump`)
      (`/Game/FPS/Core/PilotParkourMovement.Jump Event` (`self.ParkourMovement`))))
  (:`Completed`
    (`self.StopJumping`)))

(event `self.OnLanded`
  (params (Hit :type "HitResult Structure (by ref)"))
  ;[1 1 1] Player: Pilot Movement Mechanics
  ;;[1 1 1] Pilot Jumping
  (`/Game/FPS/Core/PilotParkourMovement.Land Event` (`self.ParkourMovement`)))

(event `EnhancedInput|/Game/FPS/Data/IA_PilotRun`
  (params (ActionValue :type Boolean) (ElapsedSeconds :type "Float (double-precision)") (TriggeredSeconds :type "Float (double-precision)") (InputAction :type "InputAction Object Reference" :default "/Game/FPS/Data/IA_PilotRun.IA_PilotRun"))
  (bind _returnvalue (`self.K2_GetActorLocation`))
  (bind _returnvalue_2 (`self.K2_GetActorLocation`))
  (bind _returnvalue_3 (`self.K2_GetActorLocation`))
  (bind _returnvalue_4 (`self.K2_GetActorLocation`))
  (bind _returnvalue_5 (`self.K2_GetActorLocation`))
  ;[1 1 1] Player: Pilot Movement Mechanics
  ;;[1 1 1] Pilot Running
  (:`Started`
    (if (`/Game/FPS/Core/PilotParkourMovement.bSlideInputDelay` (`self.ParkourMovement`))
      _
      (elif (`|EnumEquality` (`/Game/FPS/Core/PilotParkourMovement.eCurrentParkourMovementMode` (`self.ParkourMovement`)) "NewEnumerator0")
        (bind (_outhit _returnvalue_6) (`KismetSystemLibrary.LineTraceSingle` _returnvalue_4 (+ _returnvalue_4 (* (`self.GetActorUpVector`) 88.0)) "TraceTypeQuery1" :!label _label_3))
        (if _returnvalue_6
          (`/Game/FPS/Core/PilotParkourMovement.CrouchStart` (`self.ParkourMovement`) :!label _label_4)
          (else
            (`/Game/FPS/Core/PilotParkourMovement.Parkour Sprint Event` (`self.ParkourMovement`))
            (set `/Game/FPS/Core/PilotParkourMovement.bSprintQueued` true (`self.ParkourMovement`))))
        (else
          (bind (_outhit_2 _returnvalue_7) (`KismetSystemLibrary.LineTraceSingle` _returnvalue (+ _returnvalue (* (`self.GetActorUpVector`) 120.0) (* (`self.GetActorForwardVector`) (`CapsuleComponent.GetScaledCapsuleRadius` (`self.CapsuleComponent`)))) "TraceTypeQuery1"))
          (if _returnvalue_7
            (goto _label_4)
            (else
              (bind (_outhit_3 _returnvalue_8) (`KismetSystemLibrary.LineTraceSingle` _returnvalue_2 (+ _returnvalue_2 (* (`self.GetActorUpVector`) 120.0) (* (`self.GetActorForwardVector`) (* (`CapsuleComponent.GetScaledCapsuleRadius` (`self.CapsuleComponent`)) -1.0))) "TraceTypeQuery1"))
              (if _returnvalue_8
                (goto _label_4)
                (else
                  (bind (_outhit_4 _returnvalue_9) (`KismetSystemLibrary.LineTraceSingle` _returnvalue_3 (+ _returnvalue_3 (* (`self.GetActorUpVector`) 120.0) (* (`self.GetActorRightVector`) (`CapsuleComponent.GetScaledCapsuleRadius` (`self.CapsuleComponent`)))) "TraceTypeQuery1"))
                  (if _returnvalue_9
                    (goto _label_4)
                    (else
                      (bind (_outhit_5 _returnvalue_10) (`KismetSystemLibrary.LineTraceSingle` _returnvalue_5 (+ _returnvalue_5 (* (`self.GetActorUpVector`) 120.0) (* (`self.GetActorRightVector`) (* (`CapsuleComponent.GetScaledCapsuleRadius` (`self.CapsuleComponent`)) -1.0))) "TraceTypeQuery1"))
                      (if _returnvalue_10
                        (goto _label_4)
                        (else
                          (goto _label_3))))))))))))))

(event `CameraFOVRun`
  ;[1 1 1] Player: Pilot Movement Mechanics
  ;;[1 1 1] Pilot Running
  (if (not (`NavMovementComponent.IsFalling` (`self.CharacterMovement`)))
    ;;;[1 1 1] FOVAdjust
    (switch `/Game/FPS/Core/Enums/E_ParkourMovementType` (`/Game/FPS/Core/PilotParkourMovement.eCurrentParkourMovementMode` (`self.ParkourMovement`))
      (:`NewEnumerator0`
        ;;;[1 1 1] TODO: Make FOV Change based off of speed instead
        ;;;;[1 1 1] Adjust for FOV
        (bind (_direction _fovsmooth) (`Timeline|RunTimeline` :!via `Reverse` :!label _label_5)
          (:`Update`
            (`CameraComponent.SetFieldOfView` (`self.Camera`) _fovsmooth))))
      (:`NewEnumerator4`
        (goto _label_5 :!via `Reverse`))
      (:`NewEnumerator5`
        (goto _label_5 :!via `Reverse`))
      (:`NewEnumerator7`
        (goto _label_5 :!via `Reverse`))
      (:`NewEnumerator8`
        (goto _label_5)))))

(event `EnhancedInput|/Game/FPS/Data/IA_PilotCrouch`
  (params (ActionValue :type Boolean) (ElapsedSeconds :type "Float (double-precision)") (TriggeredSeconds :type "Float (double-precision)") (InputAction :type "InputAction Object Reference" :default "/Game/FPS/Data/IA_PilotCrouch.IA_PilotCrouch"))
  ;[1 1 1] Player: Pilot Movement Mechanics
  ;;[1 1 1] Pilot Crouching Activation
  (:`Started`
    (`/Game/FPS/Core/PilotParkourMovement.Parkour Crouch Slide Event` (`self.ParkourMovement`))))

(event `CameraSmoothCrouch`
  (bind _returnvalue (`self.K2_GetActorLocation`))
  (bind _pivot (`self.Pivot`))
  (bind _returnvalue_2 (`SceneComponent.GetRelativeTransform` _pivot))
  ;[1 1 1] Player: Pilot Movement Mechanics
  ;;[1 1 1] Pilot Crouching Activation
  (switch `/Game/FPS/Core/Enums/E_ParkourMovementType` (`/Game/FPS/Core/PilotParkourMovement.eCurrentParkourMovementMode` (`self.ParkourMovement`))
    (:`NewEnumerator0`
      ;;;[1 1 1] Crouch Speed
      (bind (_direction _halfheight) (`Timeline|Timeline` :!via `Reverse` :!label _label_6)
        (:`Update`
          (bind (_outhit _returnvalue_3) (`KismetSystemLibrary.LineTraceSingle` _returnvalue (+ _returnvalue (* (`self.GetActorUpVector`) 88.0)) "TraceTypeQuery1"))
          (if _returnvalue_3
            (`/Game/FPS/Core/PilotParkourMovement.CrouchStart` (`self.ParkourMovement`)))
          (`CapsuleComponent.SetCapsuleHalfHeight` (`self.CapsuleComponent`) _halfheight false)
          (`SceneComponent.K2_SetRelativeTransform` _pivot (`KismetMathLibrary.MakeTransform` (`KismetMathLibrary.MakeVector` (.x (.location _returnvalue_2)) (.y (.location _returnvalue_2)) _halfheight) (.rotation _returnvalue_2) (.scale _returnvalue_2)) false true))))
    (:`NewEnumerator1`
      (goto _label_6 :!via `Reverse`))
    (:`NewEnumerator2`
      (goto _label_6 :!via `Reverse`))
    (:`NewEnumerator3`
      (goto _label_6 :!via `Reverse`))
    (:`NewEnumerator5`
      (goto _label_6 :!via `Reverse`))
    (:`NewEnumerator6`
      (goto _label_6))
    (:`NewEnumerator7`
      (goto _label_6))
    (:`NewEnumerator8`
      (goto _label_6 :!via `Reverse`))))

(event `self.K2_OnMovementModeChanged`
  (params (PrevMovementMode :type "EMovementMode Enum" :default "MOVE_None") (NewMovementMode :type "EMovementMode Enum" :default "MOVE_None") (PrevCustomMode :type Byte) (NewCustomMode :type Byte))
  ;[1 1 1] Player: Pilot Movement Mechanics
  ;;[1 1 1] Update Movement State Enum
  (`/Game/FPS/Core/PilotParkourMovement.MovementChanged` (`self.ParkourMovement`) PrevMovementMode NewMovementMode))

(event `CheckWallDistance`
  (bind _camera (`self.Camera`))
  ;[1 1 1] Player: Pilot Weapon Mechanics
  ;;[1 1 1] Check if close to wall (for moving weapon away from wall when too close)
  (bind (_outhit _returnvalue) (`KismetSystemLibrary.LineTraceSingle` (`SceneComponent.K2_GetComponentLocation` (`self.Camera`)) (+ (`SceneComponent.K2_GetComponentLocation` _camera) (* (`SceneComponent.GetForwardVector` _camera) (120.0 120.0 120.0))) "TraceTypeQuery1"))
  (set `self.bCloseToWall` _returnvalue))

(event `HolsterToggle`
  ;[1 1 1] Player: Pilot Weapon Mechanics
  ;;[1 1 1] Stow Weapon
  (set `self.bEquiped` (not (`self.bEquiped`)))
  (`|PlayMontage` null (select `bool` (`self.bEquiped`) :`false` "/Game/FPS/Art/AssaultRifle/Animations/AM_FP_AssaultRifle_Holster.AM_FP_AssaultRifle_Holster" :`true` "/Game/FPS/Art/AssaultRifle/Animations/AM_FP_AssaultRifle_Equip.AM_FP_AssaultRifle_Equip" :!type "AnimMontage Object Reference")))

(event `EnhancedInput|/Game/FPS/Data/IA_PilotHolster`
  (params (ActionValue :type Boolean) (ElapsedSeconds :type "Float (double-precision)") (TriggeredSeconds :type "Float (double-precision)") (InputAction :type "InputAction Object Reference" :default "/Game/FPS/Data/IA_PilotHolster.IA_PilotHolster"))
  ;[1 1 1] Player: Pilot Weapon Mechanics
  ;;[1 1 1] Stow Weapon
)

(event `SpawnInventory`
  ;[1 1 1] Weapon Inventory
)

(event `self.ReceiveActorBeginOverlap`
  (params (OtherActor :type "Actor Object Reference"))
  ;[1 1 1] BALL PICKUP
  (if (not (== OtherActor "/Game/10SECOND/Gameplay/BP_THEBALLStatic.BP_THEBALLStatic"))
    (set `self.bBallCanBePickedUp` true)))

(event `self.ReceiveActorEndOverlap`
  (params (OtherActor :type "Actor Object Reference"))
  ;[1 1 1] BALL PICKUP
  (if (not (== OtherActor "/Game/10SECOND/Gameplay/BP_THEBALLStatic.BP_THEBALLStatic"))
    (set `self.bBallCanBePickedUp` false)))

(event `EnhancedInput|/Game/FPS/Data/IA_PilotAim`
  (params (ActionValue :type Boolean) (ElapsedSeconds :type "Float (double-precision)") (TriggeredSeconds :type "Float (double-precision)") (InputAction :type "InputAction Object Reference" :default "/Game/FPS/Data/IA_PilotAim.IA_PilotAim"))
  (bind _capsulecomponent (`self.CapsuleComponent`))
  ;[1 1 1] Picking up / Catching / Dropping the Ball (Right Click)
  (:`Triggered`
    (if (`self.bBallCanBePickedUp`)
      (`self.K2_DestroyActor` (`PrimitiveComponent.GetOverlappingActors` _capsulecomponent "/Game/10SECOND/Gameplay/BP_THEBALLStatic.BP_THEBALLStatic_C"))
      (`self.K2_DestroyActor` (`PrimitiveComponent.GetOverlappingActors` _capsulecomponent "/Game/10SECOND/Gameplay/BP_THEBALLMove1.BP_THEBALLMove1_C"))
      (`self.K2_DestroyActor` (`PrimitiveComponent.GetOverlappingActors` _capsulecomponent "/Game/10SECOND/Gameplay/BP_THEBALLMove2.BP_THEBALLMove2_C"))
      (`self.K2_DestroyActor` (`PrimitiveComponent.GetOverlappingActors` _capsulecomponent "/Game/10SECOND/Gameplay/BP_THEBALLMove3.BP_THEBALLMove3_C"))
      (set `self.bHoldingTheBall` true)
      (else
        (`/Engine/EditorBlueprintResources/StandardMacros.DoOnce` false
          (:`Completed`
            (if (`self.bHoldingTheBall`)
              (set `self.bHoldingTheBall` false)
              (`|SpawnActorFromClass` "/Game/10SECOND/Gameplay/BP_THEBALLStatic.BP_THEBALLStatic_C" (`SceneComponent.K2_GetComponentToWorld` (`self.Camera`)) "AlwaysSpawn" "MultiplyWithRoot" null null))))))))

(event `EnhancedInput|/Game/FPS/Data/IA_PilotShoot`
  (params (ActionValue :type Boolean) (ElapsedSeconds :type "Float (double-precision)") (TriggeredSeconds :type "Float (double-precision)") (InputAction :type "InputAction Object Reference" :default "/Game/FPS/Data/IA_PilotShoot.IA_PilotShoot"))
  ;[1 1 1] Shoot (Left Click)
  (:`Triggered`
    (set `self.ChargeTimeElapsed Seconds` ElapsedSeconds))
  (:`Completed`
    (if (`self.bHoldingTheBall`)
      (set `self.bHoldingTheBall` false)
      (if (>= ElapsedSeconds (`self.FullChargeThrowTime`))
        (bind _returnvalue (`|SpawnActorFromClass` "/Game/10SECOND/Gameplay/BP_THEBALLMove3.BP_THEBALLMove3_C" (`SceneComponent.K2_GetComponentToWorld` (`self.Camera`)) "AlwaysSpawn" "MultiplyWithRoot" null null))
        (`KismetSystemLibrary.PrintString` "level3")
        (elif (>= ElapsedSeconds (`self.NoChargeThrowTime`))
          (bind _returnvalue_2 (`|SpawnActorFromClass` "/Game/10SECOND/Gameplay/BP_THEBALLMove2.BP_THEBALLMove2_C" (`SceneComponent.K2_GetComponentToWorld` (`self.Camera`)) "AlwaysSpawn" "MultiplyWithRoot" null null))
          (`KismetSystemLibrary.PrintString` "level2")
          (elif (< ElapsedSeconds (`self.NoChargeThrowTime`))
            (`|PlayMontage` (`self.DroneCharacter`) "/Game/Art/Animations/Drone/DroneCharacter/FP_RevolverAnimations/AM_FireRevolverADS.AM_FireRevolverADS"
              (:`then`
                (bind _returnvalue_3 (`|SpawnActorFromClass` "/Game/10SECOND/Gameplay/BP_THEBALLMove1.BP_THEBALLMove1_C" (`SceneComponent.K2_GetComponentToWorld` (`self.Camera`)) "AlwaysSpawn" "MultiplyWithRoot" null null))
                (`KismetSystemLibrary.PrintString` "level1")))))))))

(event `EnhancedInput|/Game/FPS/Data/IA_PilotReload`
  (params (ActionValue :type Boolean) (ElapsedSeconds :type "Float (double-precision)") (TriggeredSeconds :type "Float (double-precision)") (InputAction :type "InputAction Object Reference" :default "/Game/FPS/Data/IA_PilotReload.IA_PilotReload"))
  ; BALL RECALL ON/OFF
  (:`Started`
    ;; Starts as OFF
    (`/Engine/EditorBlueprintResources/StandardMacros.FlipFlop`
      (:`A`
        (set `self.bRecall` true)
        (`KismetSystemLibrary.PrintString` "On")
        (`GameModeBase.ResetLevel` (`GameplayStatics.GetGameMode`)))
      (:`B`
        (set `self.bRecall` false)
        (`KismetSystemLibrary.PrintString` "Off")))))

(event `TIMERSTART`
  ; TIMER START (Starts when players presses WASD)
  (set `self.bTimerStart` true))

(event `TimerDone`
  (if (`self.TimerFinished`)
    (`Controller.SetIgnoreMoveInput` (`GameplayStatics.GetPlayerController` 0) true)))

(fn `UserConstructionScript`)