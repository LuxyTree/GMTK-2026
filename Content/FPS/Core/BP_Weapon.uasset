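; BP_Weapon is the first-person assault rifle actor that supplies the weapon-side visuals for shooting and reloading.
; Shoot plays the fire montage on the rifle skeletal mesh and spawns a BP_Casing at its ejection socket, with the casing set to ignore the player character when moving.
; Reload plays the reload montage to animate the magazine.
; It contains no projectile, damage or ammo logic.
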(event `/Game/FPS/Core/BPI_Weapon.Shoot`
  ;[1 1 1] Supporting AssaultRifle Firing Animations
  ;;[1 1 1] Eject Bullet Casing + Play Rack Movement on Fire
  (`|PlayMontage` (`self.SK_AssaultRifle`) "/Game/FPS/Art/AssaultRifle/Animations/AM_FP_WEP_AssaulRifle_Fire.AM_FP_WEP_AssaulRifle_Fire"
    (:`then`
      (bind _returnvalue (`|SpawnActorFromClass` "/Game/FPS/Core/BP_Casing.BP_Casing_C" (`SceneComponent.GetSocketTransform` (`self.SK_AssaultRifle`) "SOCKET_Ejection" "RTS_World") "AlwaysSpawn" "MultiplyWithRoot" null null))
      (`PrimitiveComponent.IgnoreActorWhenMoving` (`/Game/FPS/Core/BP_Casing.CasingMesh` _returnvalue) (`GameplayStatics.GetPlayerCharacter` 0) true))))

(event `/Game/FPS/Core/BPI_Weapon.Reload`
  ;[1 1 1] Supporting AssaultRifle Firing Animations
  ;;[1 1 1] Animate Magazine
  (`|PlayMontage` (`self.SK_AssaultRifle`) "/Game/FPS/Art/AssaultRifle/Animations/AM_FP_WEP_AssaultRifle_Reload.AM_FP_WEP_AssaultRifle_Reload"))

(fn `UserConstructionScript`)