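; First-person player mech character handling look, movement, jump, boost, crouch, shooting, reloading and hatch interaction, and creating the mech HUD.
; Enhanced Input events forward to the MechMovement parkour component, whose mode drives FOV and crouch-height timelines, while overhead traces force crouching.
; Spawned weapons attach to the arms, and a delay loop fires bullets from the camera unless sprinting, vertical wall-running, reloading, empty, holstered or near a wall.
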(event `self.ReceiveBeginPlay`
  (bind _returnvalue (`GameplayStatics.GetPlayerCameraManager` 0))
  ;[1 1 1] Initialize Mech
  (`self.SetupMechControls`)
  (`self.SpawnInventory`)
  (`self.CreateMechHUD`)
  (`self.HolsterToggle`)
  (`/Game/FPS/Core/MechMovement.InitializeMech` (`self.MechMovement`) self)
  ;;[1 1 1] Mech Look Up/Down Max
  (set `PlayerCameraManager.ViewPitchMin` -80.0 _returnvalue)
  (set `PlayerCameraManager.ViewPitchMax` 80.0 _returnvalue))

(event `CreateMechHUD`
  ;[1 1 1] Create HUD
  (bind _returnvalue (`|CreateWidget` "/Game/FPS/Core/WBP_MechUI.WBP_MechUI_C" (`GameplayStatics.GetPlayerController` 0)))
  (`UserWidget.AddToViewport` _returnvalue 0))

(event `self.ReceiveTick`
  (params (DeltaSeconds :type "Float (single-precision)"))
  ;[1 1 1] Update Event
  (`self.MechRotationPivot`)
  (`self.CheckWallDistance`)
  (`self.CameraFOVRun`)
  (set `self.MechSpeedometer` (`KismetMathLibrary.VSize` (`self.GetVelocity`))))

(event `EnhancedInput|/Game/FPS/Data/IA_MechTest`
  (params (ActionValue :type Boolean) (ElapsedSeconds :type "Float (double-precision)") (TriggeredSeconds :type "Float (double-precision)") (InputAction :type "InputAction Object Reference" :default "/Game/FPS/Data/IA_MechTest.IA_MechTest"))
  ;[1 1 1] Update Event
  ;;[1 1 1] Debug (T)
  (:`Triggered`
    (`KismetSystemLibrary.PrintString` "Hello")))

(event `SetupMechControls`
  ;[1 1 1] Player: Mech Movement Mechanics
  ;;[1 1 1] Link Correct Movement Mapping (Happens in Player Controller now)
)

(event `EnhancedInput|/Game/FPS/Data/IA_MechCamera`
  (params (ActionValue :type "Vector2D Structure") (ElapsedSeconds :type "Float (double-precision)") (TriggeredSeconds :type "Float (double-precision)") (InputAction :type "InputAction Object Reference" :default "/Game/FPS/Data/IA_MechCamera.IA_MechCamera"))
  (bind (_x _y) (`KismetMathLibrary.BreakVector2D` (`self.MouseInput`)))
  ;[1 1 1] Player: Mech Movement Mechanics
  ;;[1 1 1] Mouse Camera Movement
  (:`Triggered`
    (set `self.MouseInput` ActionValue :!label _label)
    (`self.AddControllerPitchInput` (* _y -1.0))
    (`self.AddControllerYawInput` _x))
  (:`Completed`
    (goto _label)))

(event `MechRotationPivot`
  ;[1 1 1] Player: Mech Movement Mechanics
  ;;[1 1 1] Mech Rotation Pivot (Allows the players arms to move same as the mouse)
  (`SceneComponent.K2_SetRelativeRotation` (`self.Pivot`) (`KismetMathLibrary.MakeRotator` 0.0 (.pitch (`self.GetControlRotation`))) false false))

(event `EnhancedInput|/Game/FPS/Data/IA_MechMovement`
  (params (ActionValue :type "Vector2D Structure") (ElapsedSeconds :type "Float (double-precision)") (TriggeredSeconds :type "Float (double-precision)") (InputAction :type "InputAction Object Reference" :default "/Game/FPS/Data/IA_MechMovement.IA_MechMovement"))
  (bind (_x _y) (`KismetMathLibrary.BreakVector2D` (`self.MoveInput`)))
  ;[1 1 1] Player: Mech Movement Mechanics
  ;;[1 1 1] WASD Mech Movement
  (:`Triggered`
    (set `self.MoveInput` ActionValue :!label _label_2)
    (`self.AddMovementInput` (* (`self.GetActorForwardVector`) _y))
    (`self.AddMovementInput` (* (`self.GetActorRightVector`) _x))
    (`/Game/FPS/Core/MechMovement.MechSpeedConservation` (`self.MechMovement`))
    (`KismetSystemLibrary.Delay` (`self.Accel/Decel Determination Time`))
    (set `/Game/FPS/Core/MechMovement.LastSpeed` (`self.MechSpeedometer`) (`self.MechMovement`)))
  (:`Completed`
    (goto _label_2)))

(event `EnhancedInput|/Game/FPS/Data/IA_MechJump`
  (params (ActionValue :type Boolean) (ElapsedSeconds :type "Float (double-precision)") (TriggeredSeconds :type "Float (double-precision)") (InputAction :type "InputAction Object Reference" :default "/Game/FPS/Data/IA_MechJump.IA_MechJump"))
  ;[1 1 1] Player: Mech Movement Mechanics
  ;;[1 1 1] Mech Jumping
  (:`Started`
    (`self.Jump`)
    (`/Game/FPS/Core/MechMovement.Jump Event` (`self.MechMovement`)))
  (:`Completed`
    (`self.StopJumping`)))

(event `self.OnLanded`
  (params (Hit :type "HitResult Structure (by ref)"))
  ;[1 1 1] Player: Mech Movement Mechanics
  ;;[1 1 1] Mech Jumping
  (`/Game/FPS/Core/MechMovement.Land Event` (`self.MechMovement`)))

(event `EnhancedInput|/Game/FPS/Data/IA_MechBoost`
  (params (ActionValue :type Boolean) (ElapsedSeconds :type "Float (double-precision)") (TriggeredSeconds :type "Float (double-precision)") (InputAction :type "InputAction Object Reference" :default "/Game/FPS/Data/IA_MechBoost.IA_MechBoost"))
  (bind _returnvalue (`self.K2_GetActorLocation`))
  (bind _returnvalue_2 (`self.K2_GetActorLocation`))
  (bind _returnvalue_3 (`self.K2_GetActorLocation`))
  (bind _returnvalue_4 (`self.K2_GetActorLocation`))
  (bind _returnvalue_5 (`self.K2_GetActorLocation`))
  (bind _mechmovement (`self.MechMovement`))
  ;[1 1 1] Player: Mech Movement Mechanics
  ;;[1 1 1] Mech Boost
  (:`Started`
    (if (`|EnumEquality` (`/Game/FPS/Core/MechMovement.eCurrentParkourMovementMode` (`self.MechMovement`)) "NewEnumerator0")
      (bind (_outhit _returnvalue_6) (`KismetSystemLibrary.LineTraceSingle` _returnvalue_4 (+ _returnvalue_4 (* (`self.GetActorUpVector`) 88.0)) "TraceTypeQuery1" :!label _label_3))
      (if _returnvalue_6
        (`/Game/FPS/Core/MechMovement.CrouchStart` (`self.MechMovement`) :!label _label_4)
        (else
          (`/Game/FPS/Core/MechMovement.Parkour Sprint Event` _mechmovement)
          (set `/Game/FPS/Core/MechMovement.bSprintQueued` true _mechmovement)))
      (else
        (bind (_outhit_2 _returnvalue_7) (`KismetSystemLibrary.LineTraceSingle` _returnvalue (+ _returnvalue (* (`self.GetActorUpVector`) 120.0) (* (`self.GetActorForwardVector`) (`CapsuleComponent.GetScaledCapsuleRadius` (`self.CapsuleComponent`)))) "TraceTypeQuery1"))
        (if _returnvalue_7
          (goto _label_4)
          (else
            (bind (_outhit_3 _returnvalue_8) (`KismetSystemLibrary.LineTraceSingle` _returnvalue_2 (+ _returnvalue_2 (* (`self.GetActorUpVector`) 120.0) (* (`self.GetActorForwardVector`) (* (`CapsuleComponent.GetScaledCapsuleRadius` (`self.CapsuleComponent`)) -1.0))) "TraceTypeQuery1"))
            (if _returnvalue_8
              (goto _label_4)
              (else
                (bind (_outhit_4 _returnvalue_9) (`KismetSystemLibrary.LineTraceSingle` _returnvalue_3 (+ _returnvalue_3 (* (`self.GetActorUpVector`) 120.0) (* (`self.GetActorRightVector`) (`CapsuleComponent.GetScaledCapsuleRadius` (`self.CapsuleComponent`)))) "TraceTypeQuery1"))
                (if _returnvalue_9
                  (goto _label_4)
                  (else
                    (bind (_outhit_5 _returnvalue_10) (`KismetSystemLibrary.LineTraceSingle` _returnvalue_5 (+ _returnvalue_5 (* (`self.GetActorUpVector`) 120.0) (* (`self.GetActorRightVector`) (* (`CapsuleComponent.GetScaledCapsuleRadius` (`self.CapsuleComponent`)) -1.0))) "TraceTypeQuery1"))
                    (if _returnvalue_10
                      (goto _label_4)
                      (else
                        (goto _label_3)))))))))))))

(event `CameraFOVRun`
  ;[1 1 1] Player: Mech Movement Mechanics
  ;;[1 1 1] Mech Boost
  (if (not (`NavMovementComponent.IsFalling` (`self.CharacterMovement`)))
    ;;;[1 1 1] FOVAdjust
    (switch `/Game/FPS/Core/Enums/E_ParkourMovementType` (`/Game/FPS/Core/MechMovement.eCurrentParkourMovementMode` (`self.MechMovement`))
      (:`NewEnumerator0`
        ;;;[1 1 1] TODO: Make FOV Change based off of speed instead
        ;;;;[1 1 1] Adjust for FOV
        (bind (_direction _fovsmooth) (`Timeline|RunTimeline` :!via `Reverse` :!label _label_5)
          (:`Update`
            (`CameraComponent.SetFieldOfView` (`self.Camera`) _fovsmooth))))
      (:`NewEnumerator4`
        (goto _label_5 :!via `Reverse`))
      (:`NewEnumerator5`
        (goto _label_5 :!via `Reverse`))
      (:`NewEnumerator7`
        (goto _label_5 :!via `Reverse`))
      (:`NewEnumerator8`
        (goto _label_5)))))

(event `EnhancedInput|/Game/FPS/Data/IA_MechCrouch`
  (params (ActionValue :type Boolean) (ElapsedSeconds :type "Float (double-precision)") (TriggeredSeconds :type "Float (double-precision)") (InputAction :type "InputAction Object Reference" :default "/Game/FPS/Data/IA_MechCrouch.IA_MechCrouch"))
  ;[1 1 1] Player: Mech Movement Mechanics
  ;;[1 1 1] Mech Crouching Activation
  (:`Started`
    (`/Game/FPS/Core/MechMovement.Mech Crouch Event` (`self.MechMovement`))))

(event `CameraSmoothCrouch`
  (bind _returnvalue (`self.K2_GetActorLocation`))
  (bind _pivot (`self.Pivot`))
  (bind _returnvalue_2 (`SceneComponent.GetRelativeTransform` _pivot))
  ;[1 1 1] Player: Mech Movement Mechanics
  ;;[1 1 1] Mech Crouching Activation
  (switch `/Game/FPS/Core/Enums/E_ParkourMovementType` (`/Game/FPS/Core/MechMovement.eCurrentParkourMovementMode` (`self.MechMovement`))
    (:`NewEnumerator0`
      ;;;[1 1 1] Crouch Speed
      (bind (_direction _halfheight) (`Timeline|Timeline` :!via `Reverse` :!label _label_6)
        (:`Update`
          (bind (_outhit _returnvalue_3) (`KismetSystemLibrary.LineTraceSingle` _returnvalue (+ _returnvalue (* (`self.GetActorUpVector`) 1000.0)) "TraceTypeQuery1"))
          (if _returnvalue_3
            (`/Game/FPS/Core/MechMovement.CrouchStart` (`self.MechMovement`)))
          (`CapsuleComponent.SetCapsuleHalfHeight` (`self.CapsuleComponent`) _halfheight false)
          (`SceneComponent.K2_SetRelativeTransform` _pivot (`KismetMathLibrary.MakeTransform` (`KismetMathLibrary.MakeVector` (.x (.location _returnvalue_2)) (.y (.location _returnvalue_2)) _halfheight) (.rotation _returnvalue_2) (.scale _returnvalue_2)) false true))))
    (:`NewEnumerator1`
      (goto _label_6 :!via `Reverse`))
    (:`NewEnumerator2`
      (goto _label_6 :!via `Reverse`))
    (:`NewEnumerator3`
      (goto _label_6 :!via `Reverse`))
    (:`NewEnumerator5`
      (goto _label_6 :!via `Reverse`))
    (:`NewEnumerator6`
      (goto _label_6))
    (:`NewEnumerator7`
      (goto _label_6))
    (:`NewEnumerator8`
      (goto _label_6 :!via `Reverse`))))

(event `self.K2_OnMovementModeChanged`
  (params (PrevMovementMode :type "EMovementMode Enum" :default "MOVE_None") (NewMovementMode :type "EMovementMode Enum" :default "MOVE_None") (PrevCustomMode :type Byte) (NewCustomMode :type Byte))
  ;[1 1 1] Player: Mech Movement Mechanics
  ;;[1 1 1] Update Movement State Enum
  (`/Game/FPS/Core/MechMovement.MovementChanged` (`self.MechMovement`) PrevMovementMode NewMovementMode))

(event `EnhancedInput|/Game/FPS/Data/IA_MechAim`
  (params (ActionValue :type Boolean) (ElapsedSeconds :type "Float (double-precision)") (TriggeredSeconds :type "Float (double-precision)") (InputAction :type "InputAction Object Reference" :default "/Game/FPS/Data/IA_MechAim.IA_MechAim"))
  ;[1 1 1] Mech: Mech Weapon Mechanics
  ;;[1 1 1] Aiming
  (:`Triggered`
    (set `self.bAiming` true))
  (:`Completed`
    (set `self.bAiming` false)))

(event `CheckWallDistance`
  (bind _camera (`self.Camera`))
  ;[1 1 1] Mech: Mech Weapon Mechanics
  ;;[1 1 1] Check if close to wall (for moving weapon away from wall when too close)
  (bind (_outhit _returnvalue) (`KismetSystemLibrary.LineTraceSingle` (`SceneComponent.K2_GetComponentLocation` (`self.Camera`)) (+ (`SceneComponent.K2_GetComponentLocation` _camera) (* (`SceneComponent.GetForwardVector` _camera) (120.0 120.0 120.0))) "TraceTypeQuery1"))
  (set `self.bCloseToWall` _returnvalue))

(event `EnhancedInput|/Game/FPS/Data/IA_MechShoot`
  (params (ActionValue :type Boolean) (ElapsedSeconds :type "Float (double-precision)") (TriggeredSeconds :type "Float (double-precision)") (InputAction :type "InputAction Object Reference" :default "/Game/FPS/Data/IA_MechShoot.IA_MechShoot"))
  ;[1 1 1] Mech: Mech Weapon Mechanics
  ;;[1 1 1] Shoot
  (:`Triggered`
    (`/Engine/EditorBlueprintResources/StandardMacros.DoOnce` false :!label _label_7
      (:`Completed`
        (set `self.bHoldingShoot` true)
        (if (and (and (and (and (`self.bHoldingShoot`) (not (`|EnumEquality` (`/Game/FPS/Core/MechMovement.eCurrentParkourMovementMode` (`self.MechMovement`)) "NewEnumerator8")) (not (`self.bCloseToWall`)) (not (`|EnumEquality` (`/Game/FPS/Core/MechMovement.eCurrentParkourMovementMode` (`self.MechMovement`)) "NewEnumerator3"))) (> (`self.CurrentAmmunition`) 0)) (not (`self.bReloading`))) (`self.bEquiped`)) :!label _label_8
          (message `/Game/FPS/Core/BPI_Weapon.Shoot` (`|GetArrayItem` (`self.InventoryActive(EquipedWeapons)`) (`self.EquippedWeaponIndex`)))
          (`|PlayMontage` (`self.CharacterArms`) "/Game/FPS/Art/AssaultRifle/Animations/AM_FP_AssaultRifle_Fire.AM_FP_AssaultRifle_Fire"
            (:`then`
              (bind _returnvalue (`|SpawnActorFromClass` "/Game/FPS/Core/BP_MechBullet.BP_MechBullet_C" (`SceneComponent.K2_GetComponentToWorld` (`self.Camera`)) "AlwaysSpawn" "MultiplyWithRoot" null null))
              (`PrimitiveComponent.IgnoreActorWhenMoving` (`self.CapsuleComponent`) _returnvalue true)
              (`PrimitiveComponent.IgnoreActorWhenMoving` (`/Game/FPS/Core/BP_MechBullet.Sphere` _returnvalue) self true)
              (`GameplayStatics.SpawnEmitterAttached` "/Game/StarterContent/Particles/P_Explosion.P_Explosion" (`Actor.RootComponent` (`|GetArrayItem` (`self.InventoryActive(EquipedWeapons)`) (`self.EquippedWeaponIndex`))) "None" (0.0 90.0 0.0) (struct :`Pitch` 180.0 :`Yaw` 180.0 :`Roll` 180.0) (0.05 0.05 0.05) "SnapToTargetIncludingScale")
              (set `self.CurrentAmmunition` (- (`self.CurrentAmmunition`) 1))
              (`KismetSystemLibrary.Delay` (`self.FireDelay`))
              (goto _label_8)))))))
  (:`Completed`
    (set `self.bHoldingShoot` false)
    (goto _label_7 :!via `Reset`)))

(event `EnhancedInput|/Game/FPS/Data/IA_MechReload`
  (params (ActionValue :type Boolean) (ElapsedSeconds :type "Float (double-precision)") (TriggeredSeconds :type "Float (double-precision)") (InputAction :type "InputAction Object Reference" :default "/Game/FPS/Data/IA_MechReload.IA_MechReload"))
  ;[1 1 1] Mech: Mech Weapon Mechanics
  ;;[1 1 1] Reload
  (:`Triggered`
    (`/Engine/EditorBlueprintResources/StandardMacros.DoOnce` false :!label _label_9
      (:`Completed`
        (if (`self.bEquiped`)
          (set `self.bReloading` true)
          (`|PlayMontage` (`self.CharacterArms`) "/Game/FPS/Art/AssaultRifle/Animations/AM_FP_AssaultRifle_Reload.AM_FP_AssaultRifle_Reload"
            (:`then`
              (message `/Game/FPS/Core/BPI_Weapon.Reload` (`|GetArrayItem` (`self.InventoryActive(EquipedWeapons)`) (`self.EquippedWeaponIndex`))))
            (:`OnCompleted`
              (set `self.CurrentAmmunition` (`self.TotalAmmunition`)))
            (:`OnBlendOut`
              (set `self.bReloading` false)))))))
  (:`Completed`
    (goto _label_9 :!via `Reset`)))

(event `HolsterToggle`
  ;[1 1 1] Mech: Mech Weapon Mechanics
  ;;[1 1 1] Stow Weapon (Not used on mech)
  (set `self.bEquiped` (not (`self.bEquiped`)))
  (`|PlayMontage` (`self.CharacterArms`) (select `bool` (`self.bEquiped`) :`false` "/Game/FPS/Art/AssaultRifle/Animations/AM_FP_AssaultRifle_Holster.AM_FP_AssaultRifle_Holster" :`true` "/Game/FPS/Art/AssaultRifle/Animations/AM_FP_AssaultRifle_Equip.AM_FP_AssaultRifle_Equip" :!type "AnimMontage Object Reference")))

(event `SpawnInventory`
  ;[1 1 1] Weapon Inventory
  (for _array_element (`self.InventoryAll(AllItems)`)
    (bind _returnvalue (`|SpawnActorFromClass` _array_element (`KismetMathLibrary.MakeTransform` (0.0 0.0 0.0)) "Undefined" "MultiplyWithRoot" null null))
    (`KismetArrayLibrary.Array_Add` (`self.InventoryActive(EquipedWeapons)`) _returnvalue)
    (`self.K2_AttachToComponent` _returnvalue (`self.CharacterArms`) "ik_hand_gun" "KeepRelative" "KeepRelative" "KeepRelative" true)
    (`self.SetActorHiddenInGame` _returnvalue true))
  (`self.SetActorHiddenInGame` (`|GetArrayItem` (`self.InventoryActive(EquipedWeapons)`) (`self.EquippedWeaponIndex`)) false))

(event `self.CapsuleComponent.OnComponentBeginOverlap`
  (params (OverlappedComponent :type "PrimitiveComponent Object Reference") (OtherActor :type "Actor Object Reference") (OtherComp :type "PrimitiveComponent Object Reference") (OtherBodyIndex :type Integer) (bFromSweep :type Boolean) (SweepResult :type "HitResult Structure (by ref)")))

(event `EnhancedInput|/Game/FPS/Data/IA_MechInteract`
  (params (ActionValue :type "Vector2D Structure") (ElapsedSeconds :type "Float (double-precision)") (TriggeredSeconds :type "Float (double-precision)") (InputAction :type "InputAction Object Reference" :default "/Game/FPS/Data/IA_MechInteract.IA_MechInteract"))
  (:`Triggered`
    (bind _asbp_mech_interactable_object (cast `/Game/Missions/InvadeBunkerMissions/BP_MechInteractableObject` (stale `self.CapsuleComponent.OnComponentBeginOverlap` OtherActor)))
    (`/Engine/EditorBlueprintResources/StandardMacros.IsValid` _asbp_mech_interactable_object
      (:`Is Valid`
        (`/Game/Missions/InvadeBunkerMissions/BP_MechInteractableObject.OpenHatch` _asbp_mech_interactable_object)))))

(fn `UserConstructionScript`)