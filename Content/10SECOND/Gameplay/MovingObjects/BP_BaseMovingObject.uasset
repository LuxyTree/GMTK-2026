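; Base actor for objects that travel along a spline path, such as moving gameplay pieces.
; Each Tick advances a distance along PathSpline by MoveSpeed and MoveDirection, then snaps ObjectMesh to that world location and rotation while keeping its scale.
; Past either end of the spline, it restarts at the beginning if Loop is set, otherwise it reverses direction to ping-pong.
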(event `self.ReceiveTick`
  (params (DeltaSeconds :type "Float (single-precision)"))
  (bind _objectmesh (`self.ObjectMesh`))
  (bind _output_get (set `self.DistAlongSpline` (+ (* DeltaSeconds (`self.MoveSpeed`) (`self.MoveDirection`)) (`self.DistAlongSpline`))))
  (bind (_returnvalue_location _returnvalue_rotation) (`KismetMathLibrary.BreakTransform` (`SplineComponent.GetTransformAtDistanceAlongSpline` (`self.PathSpline`) _output_get "World" false)))
  (`SceneComponent.K2_SetWorldTransform` _objectmesh (`KismetMathLibrary.MakeTransform` _returnvalue_location _returnvalue_rotation (`SceneComponent.K2_GetComponentScale` _objectmesh)) false false)
  (if (or (>= (`self.DistAlongSpline`) (`SplineComponent.GetSplineLength` (`self.PathSpline`))) (< (`self.DistAlongSpline`) 0.0))
    (if (`self.bLoop`)
      (set `self.DistAlongSpline` 0.0)
      (elif (> (`self.MoveDirection`) 0.0)
        (set `self.MoveDirection` -1.0)
        (else
          (set `self.MoveDirection` 1.0))))))

(fn `UserConstructionScript`)