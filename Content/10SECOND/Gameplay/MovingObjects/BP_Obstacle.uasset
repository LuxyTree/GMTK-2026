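; BP_Obstacle is a hazard that makes the pilot character lose the ball on contact.
; When a capsule component of a BP_PilotCharacter begins overlapping BoxCollision while HoldingTheBall is set, it clears that flag.
; It then spawns a BP_THEBALLStatic at the character's camera transform, ignoring collisions.
; The graph itself contains no movement logic.
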(event `self.BoxCollision.OnComponentBeginOverlap`
  (params (OverlappedComponent :type "PrimitiveComponent Object Reference") (OtherActor :type "Actor Object Reference") (OtherComp :type "PrimitiveComponent Object Reference") (OtherBodyIndex :type Integer) (bFromSweep :type Boolean) (SweepResult :type "HitResult Structure (by ref)"))
  (cast `CapsuleComponent` OtherComp)
  (bind _asbp_pilot_character (cast `/Game/FPS/Core/BP_PilotCharacter` OtherActor))
  (if (`/Game/FPS/Core/BP_PilotCharacter.bHoldingTheBall` _asbp_pilot_character)
    (set `/Game/FPS/Core/BP_PilotCharacter.bHoldingTheBall` false _asbp_pilot_character)
    (`|SpawnActorFromClass` "/Game/10SECOND/Gameplay/BP_THEBALLStatic.BP_THEBALLStatic_C" (`SceneComponent.K2_GetComponentToWorld` (`/Game/FPS/Core/BP_PilotCharacter.Camera` _asbp_pilot_character)) "AlwaysSpawn" "MultiplyWithRoot" null null)))

(fn `UserConstructionScript`
  (`parent.UserConstructionScript`))