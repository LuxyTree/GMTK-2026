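; BP_THEBALLMove2 is the ball projectile, which plays a throw sound on spawn and can home back to the player.
; Each Tick reads the pilot character's Recall flag to switch projectile movement homing toward the player's capsule on or off.
; Sphere hits play one of two random bounce sounds with varied pitch, gated by a brief boolean cooldown to prevent rapid repeats.
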(event `self.ReceiveBeginPlay`
  (`GameplayStatics.PlaySound2D` "/Game/10SECOND/SFX/Throw2.Throw2" 0.5 (`KismetMathLibrary.RandomFloatInRange` 0.9 1.1) 0.0 null null))

(event `self.ReceiveTick`
  (params (DeltaSeconds :type "Float (single-precision)"))
  (`self.BallRecallToggle2`))

(event `BallRecallToggle2`
  (bind _projectilemovement (`self.ProjectileMovement`))
  (bind _asbp_pilot_character (cast `/Game/FPS/Core/BP_PilotCharacter` (`GameplayStatics.GetPlayerPawn` 0)))
  (if (`/Game/FPS/Core/BP_PilotCharacter.bRecall` _asbp_pilot_character)
    (set `ProjectileMovementComponent.bIsHomingProjectile` true _projectilemovement)
    (set `ProjectileMovementComponent.HomingTargetComponent` (`Character.CapsuleComponent` (`GameplayStatics.GetPlayerCharacter` 0)) (`self.ProjectileMovement`))
    (else
      (set `ProjectileMovementComponent.bIsHomingProjectile` false _projectilemovement))))

(event `self.Sphere.OnComponentHit`
  (params (HitComponent :type "PrimitiveComponent Object Reference") (OtherActor :type "Actor Object Reference") (OtherComp :type "PrimitiveComponent Object Reference") (NormalImpulse :type "Vector Structure") (Hit :type "HitResult Structure (by ref)"))
  (if (`KismetMathLibrary.RandomBool`)
    (if (not (`self.NewVar`))
      (`GameplayStatics.PlaySound2D` "/Game/10SECOND/SFX/BallBounce1.BallBounce1" 1.0 (`KismetMathLibrary.RandomFloatInRange` 0.9 1.1) 0.0 null null)
      (set `self.NewVar` true)
      (`KismetSystemLibrary.Delay` 0.3)
      (set `self.NewVar` false))
    (elif (not (`self.NewVar`))
      (`GameplayStatics.PlaySound2D` "/Game/10SECOND/SFX/BallBounce2.BallBounce2" 1.0 (`KismetMathLibrary.RandomFloatInRange` 0.9 1.1) 0.0 null null)
      (set `self.NewVar` true)
      (`KismetSystemLibrary.Delay` 0.3)
      (set `self.NewVar` false))))

(fn `BallRecallToggle`)

(fn `UserConstructionScript`)