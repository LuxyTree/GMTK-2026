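; BP_Launchpad is a launchpad that throws the player's pilot character when it enters the pad's box trigger.
; BeginPlay caches player 0's character as a BP_PilotCharacter.
; On overlap, if the other actor's root component has PlayerTag, it ends sprinting through the cached pilot's ParkourMovement.
; It then launches that cached pilot by LaunchVelocity, overriding vertical velocity while adding to horizontal momentum.
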(event `self.ReceiveBeginPlay`
  (bind _asbp_pilot_character (cast `/Game/FPS/Core/BP_PilotCharacter` (`GameplayStatics.GetPlayerCharacter` 0)))
  (set `self.As BP Pilot Character` _asbp_pilot_character))

(event `self.Box.OnComponentBeginOverlap`
  (params (OverlappedComponent :type "PrimitiveComponent Object Reference") (OtherActor :type "Actor Object Reference") (OtherComp :type "PrimitiveComponent Object Reference") (OtherBodyIndex :type Integer) (bFromSweep :type Boolean) (SweepResult :type "HitResult Structure (by ref)"))
  (bind _as_bp_pilot_character (`self.As BP Pilot Character`))
  (if (`ActorComponent.ComponentHasTag` (`Actor.RootComponent` OtherActor) "PlayerTag")
    (`/Game/FPS/Core/PilotParkourMovement.SprintEnd` (`/Game/FPS/Core/BP_PilotCharacter.ParkourMovement` _as_bp_pilot_character))
    (`Character.LaunchCharacter` _as_bp_pilot_character (`self.Launch Velocity`) false true)))

(fn `UserConstructionScript`)