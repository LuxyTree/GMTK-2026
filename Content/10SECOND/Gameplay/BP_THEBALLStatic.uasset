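; BP_THEBALLStatic is a ball projectile actor that homes back toward the player while the pilot character's Recall flag is set.
; Each Tick calls the BallRecallToggle0 event, which casts player pawn 0 to BP_PilotCharacter and polls Recall.
; When Recall is true, ProjectileMovement homes on the player's capsule, and when false, homing is switched off.
; The separate BallRecallToggle function is empty.
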(event `self.ReceiveBeginPlay`)

(event `self.ReceiveTick`
  (params (DeltaSeconds :type "Float (single-precision)"))
  (`self.BallRecallToggle0`))

(event `BallRecallToggle0`
  (bind _projectilemovement (`self.ProjectileMovement`))
  (bind _asbp_pilot_character (cast `/Game/FPS/Core/BP_PilotCharacter` (`GameplayStatics.GetPlayerPawn` 0)))
  (if (`/Game/FPS/Core/BP_PilotCharacter.bRecall` _asbp_pilot_character)
    (set `ProjectileMovementComponent.bIsHomingProjectile` true _projectilemovement)
    (set `ProjectileMovementComponent.HomingTargetComponent` (`Character.CapsuleComponent` (`GameplayStatics.GetPlayerCharacter` 0)) (`self.ProjectileMovement`))
    (else
      (set `ProjectileMovementComponent.bIsHomingProjectile` false _projectilemovement))))

(fn `BallRecallToggle`)

(fn `UserConstructionScript`)