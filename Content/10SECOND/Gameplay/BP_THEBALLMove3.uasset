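; BP_THEBALLMove3 is a thrown ball projectile that plays a pitch-varied throw sound on spawn.
; Hitting or overlapping a "SideObj" actor makes its ProjectileMovement home back to the player's capsule.
; Each tick, it homes on the pilot character's HOMINGTARGET while that character's HomingThrow flag is set, overriding the return target.
; Hits play one of two random bounce sounds, throttled by a short delay gate.
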(event `self.ReceiveBeginPlay`
  (`GameplayStatics.PlaySound2D` "/Game/10SECOND/SFX/Throw3.Throw3" 0.5 (`KismetMathLibrary.RandomFloatInRange` 0.9 1.1) 0.0 null null))

(event `self.ReceiveTick`
  (params (DeltaSeconds :type "Float (single-precision)"))
  (`self.HomingGoalTHrow`))

(event `self.Sphere.OnComponentHit`
  (params (HitComponent :type "PrimitiveComponent Object Reference") (OtherActor :type "Actor Object Reference") (OtherComp :type "PrimitiveComponent Object Reference") (NormalImpulse :type "Vector Structure") (Hit :type "HitResult Structure (by ref)"))
  (`|ExecutionSequence`
    (:`then_0`
      (if (`self.ActorHasTag` OtherActor "SideObj")
        (set `ProjectileMovementComponent.bIsHomingProjectile` true (`self.ProjectileMovement`) :!label _label)
        (set `ProjectileMovementComponent.HomingTargetComponent` (`Character.CapsuleComponent` (`GameplayStatics.GetPlayerCharacter` 0)) (`self.ProjectileMovement`))))
    (:`then_1`
      (if (`KismetMathLibrary.RandomBool`)
        (if (not (`self.bDelayBounceSound`))
          (`GameplayStatics.PlaySound2D` "/Game/10SECOND/SFX/BallBounce1.BallBounce1" 1.0 (`KismetMathLibrary.RandomFloatInRange` 0.9 1.1) 0.0 null null)
          (set `self.bDelayBounceSound` true)
          (`KismetSystemLibrary.Delay` 0.3)
          (set `self.bDelayBounceSound` false))
        (elif (not (`self.bDelayBounceSound`))
          (`GameplayStatics.PlaySound2D` "/Game/10SECOND/SFX/BallBounce2.BallBounce2" 1.0 (`KismetMathLibrary.RandomFloatInRange` 0.9 1.1) 0.0 null null)
          (set `self.bDelayBounceSound` true)
          (`KismetSystemLibrary.Delay` 0.3)
          (set `self.bDelayBounceSound` false))))))

(event `self.Sphere.OnComponentBeginOverlap`
  (params (OverlappedComponent :type "PrimitiveComponent Object Reference") (OtherActor :type "Actor Object Reference") (OtherComp :type "PrimitiveComponent Object Reference") (OtherBodyIndex :type Integer) (bFromSweep :type Boolean) (SweepResult :type "HitResult Structure (by ref)"))
  (if (`self.ActorHasTag` OtherActor "SideObj")
    (goto _label)))

(event `HomingGoalThrow`
  (bind _asbp_pilot_character (cast `/Game/FPS/Core/BP_PilotCharacter` (`GameplayStatics.GetPlayerPawn` 0)))
  (if (`/Game/FPS/Core/BP_PilotCharacter.HomingThrow` _asbp_pilot_character)
    (set `ProjectileMovementComponent.bIsHomingProjectile` true (`self.ProjectileMovement`))
    (set `ProjectileMovementComponent.HomingTargetComponent` (`/Game/FPS/Core/BP_PilotCharacter.HOMING TARGET` _asbp_pilot_character) (`self.ProjectileMovement`))))

(fn `BallRecallToggle`)

(fn `UserConstructionScript`)