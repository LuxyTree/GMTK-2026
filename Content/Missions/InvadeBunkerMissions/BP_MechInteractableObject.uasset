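; Bunker hatch interactable for the Invade Bunker mission (Mission 3) that only the Mech can open.
; On BeginPlay it sets the objective through GM_FPS to open the hatch with the Mech.
; Overlapping MechTriggerArea as BP_MechCharacter toggles CanInteract and the mission HUD prompt.
; OpenHatch, which has no caller here, clears the prompt, destroys the actor and advances the objective to entering the bunker with the Pilot.
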(event `self.ReceiveBeginPlay`
  (bind _asgm_fps (cast `/Game/FPS/Core/GM_FPS` (`GameplayStatics.GetGameMode`)))
  (`/Game/FPS/Core/GM_FPS.UpdateMission3(InvadeBUnker)` _asgm_fps "Open the Hatch with the Mech"))

(event `OpenHatch`
  (if (`self.bCanInteract`)
    (bind _asgm_fps (cast `/Game/FPS/Core/GM_FPS` (`GameplayStatics.GetGameMode`)))
    (`/Game/Missions/WBP_MissionHUD.CannotInteract` (`/Game/FPS/Core/GM_FPS.MissionWidgetHUD` _asgm_fps))
    (`self.K2_DestroyActor`)
    (bind _asgm_fps_2 (cast `/Game/FPS/Core/GM_FPS` (`GameplayStatics.GetGameMode`)))
    (`/Game/FPS/Core/GM_FPS.UpdateMission3(InvadeBUnker)` _asgm_fps_2 "Enter the Bunker with the Pilot")))

(event `self.MechTriggerArea.OnComponentBeginOverlap`
  (params (OverlappedComponent :type "PrimitiveComponent Object Reference") (OtherActor :type "Actor Object Reference") (OtherComp :type "PrimitiveComponent Object Reference") (OtherBodyIndex :type Integer) (bFromSweep :type Boolean) (SweepResult :type "HitResult Structure (by ref)"))
  (cast `/Game/FPS/Core/BP_MechCharacter` OtherActor)
  (set `self.bCanInteract` true)
  (bind _asgm_fps (cast `/Game/FPS/Core/GM_FPS` (`GameplayStatics.GetGameMode`)))
  (`/Game/Missions/WBP_MissionHUD.CanInteract` (`/Game/FPS/Core/GM_FPS.MissionWidgetHUD` _asgm_fps)))

(event `self.MechTriggerArea.OnComponentEndOverlap`
  (params (OverlappedComponent :type "PrimitiveComponent Object Reference") (OtherActor :type "Actor Object Reference") (OtherComp :type "PrimitiveComponent Object Reference") (OtherBodyIndex :type Integer))
  (cast `/Game/FPS/Core/BP_MechCharacter` OtherActor)
  (set `self.bCanInteract` false)
  (bind _asgm_fps (cast `/Game/FPS/Core/GM_FPS` (`GameplayStatics.GetGameMode`)))
  (`/Game/Missions/WBP_MissionHUD.CannotInteract` (`/Game/FPS/Core/GM_FPS.MissionWidgetHUD` _asgm_fps)))

(fn `UserConstructionScript`)