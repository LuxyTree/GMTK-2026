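; Mission trigger actor that completes the third pilot objective when the player interacts inside its collision volume.
; Overlap events on the pilot character toggle a CanInteract flag and show or hide the interact prompt on the GM_FPS mission HUD.
; CompleteFetchQuest(PilotM3), if interaction is allowed, hides the prompt, clears Obj3Active on the game mode, then destroys itself and any valid MechBlockerShield.
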(event `CompleteFetchQuest(PilotM3)`
  (bind _mechblockershield (`self.MechBlockerShield`))
  (if (`self.CanInteract`)
    (bind _asgm_fps (cast `/Game/FPS/Core/GM_FPS` (`GameplayStatics.GetGameMode`)))
    (`/Game/Missions/WBP_MissionHUD.CannotInteract` (`/Game/FPS/Core/GM_FPS.MissionWidgetHUD` _asgm_fps))
    (bind _asgm_fps_2 (cast `/Game/FPS/Core/GM_FPS` (`GameplayStatics.GetGameMode`)))
    (set `/Game/FPS/Core/GM_FPS.Obj3Active` false _asgm_fps_2)
    (`self.K2_DestroyActor`)
    (`/Engine/EditorBlueprintResources/StandardMacros.IsValid` _mechblockershield
      (:`Is Valid`
        (`self.K2_DestroyActor` _mechblockershield)))))

(event `self.MissionTriggerCollision.OnComponentBeginOverlap`
  (params (OverlappedComponent :type "PrimitiveComponent Object Reference") (OtherActor :type "Actor Object Reference") (OtherComp :type "PrimitiveComponent Object Reference") (OtherBodyIndex :type Integer) (bFromSweep :type Boolean) (SweepResult :type "HitResult Structure (by ref)"))
  (cast `/Game/FPS/Core/BP_PilotCharacter` OtherActor)
  (set `self.CanInteract` true)
  (bind _asgm_fps (cast `/Game/FPS/Core/GM_FPS` (`GameplayStatics.GetGameMode`)))
  (`/Game/Missions/WBP_MissionHUD.CanInteract` (`/Game/FPS/Core/GM_FPS.MissionWidgetHUD` _asgm_fps)))

(event `self.MissionTriggerCollision.OnComponentEndOverlap`
  (params (OverlappedComponent :type "PrimitiveComponent Object Reference") (OtherActor :type "Actor Object Reference") (OtherComp :type "PrimitiveComponent Object Reference") (OtherBodyIndex :type Integer))
  (cast `/Game/FPS/Core/BP_PilotCharacter` OtherActor)
  (set `self.CanInteract` false)
  (bind _asgm_fps (cast `/Game/FPS/Core/GM_FPS` (`GameplayStatics.GetGameMode`)))
  (`/Game/Missions/WBP_MissionHUD.CannotInteract` (`/Game/FPS/Core/GM_FPS.MissionWidgetHUD` _asgm_fps)))

(fn `UserConstructionScript`)